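; Player character base for Feast or Famine that handles interaction input and owns the local player's UI.
; On BeginPlay, the locally controlled pawn creates the HUD and a crafting/inventory widget wired to its inventory and crafting components.
; Interact input forwards to the interaction sensor, while menu inputs and Open/Close UI events route through AddMenu and RemoveMenu.
; These track a single active widget and switch cursor visibility and input mode.
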(event `self.ReceiveBeginPlay`
  ;[1 0.125 0.125] Begin Play Init
  (`self.Local Player Initalize`))

(event `InputAction|Interact`
  (params (Key :type "Key Structure"))
  ;[1 0.8004 0.1455] Interact
  (:`Pressed`
    (`PlayerInteractionSensor.Interact` (`self.PlayerInteractionSensor`))))

(event `InputAction|Toggle In Game Menu`
  (params (Key :type "Key Structure"))
  ;[0.2584 1 0.87] UI Management
  (:`Pressed`
    (`/Game/FeastOrFamine/UI/PlayerHUD/WBP_BasePlayerHUD.Toggle In Game Menu` (`self.Player Widget`))))

(event `InputAction|Toggle Inventory`
  (params (Key :type "Key Structure"))
  ;[0.2584 1 0.87] UI Management
  (:`Pressed`
    (if (`Widget.IsInViewport` (`self.Player Inventory Widget`))
      (`self.Remove Menu` (`self.Player Inventory Widget`))
      (else
        (bind _active_widget (`self.Active Widget`)
          (:`then`
            (`self.Remove Menu` _active_widget))
          (:`else`
            (`self.Add Menu` (`self.Player Inventory Widget`))))))))

(event `UIPlayerInterface.OpenUI`
  (params (Widget :type "CustomUserWidget Object Reference"))
  ;[0.2584 1 0.87] UI Management
  (`self.Add Menu` Widget))

(event `UIPlayerInterface.CloseUI`
  (params (Widget :type "CustomUserWidget Object Reference"))
  ;[0.2584 1 0.87] UI Management
  (`self.Remove Menu` Widget))

(event `UIPlayerInterface.CloseActiveUI`
  ;[0.2584 1 0.87] UI Management
  (bind _active_widget (`self.Active Widget`)
    (:`then`
      (`self.Remove Menu` _active_widget))
    (:`else`)))

(fn `Add Menu`
  (params (`New Widget` :type "UserWidget Object Reference"))
  (bind _active_widget (`self.Active Widget`)
    (:`then`
      (`Widget.RemoveFromParent` _active_widget)
      (set `self.Active Widget` null))
    (:`else`
      _))
  (`UserWidget.AddToViewport` `New Widget` 0)
  (bind _asplayer_controller (cast `PlayerController` (`self.GetController`)))
  (set `PlayerController.bShowMouseCursor` true _asplayer_controller)
  (`WidgetBlueprintLibrary.SetInputMode_GameAndUIEx` _asplayer_controller (`local.New Widget`))
  (set `self.Active Widget` (`local.New Widget`)))

(fn `Local Player Initalize`
  (if (`self.IsLocallyControlled`)
    (bind _returnvalue (`|CreateWidget` "/Game/FeastOrFamine/UI/PlayerHUD/WBP_BasePlayerHUD.WBP_BasePlayerHUD_C" (`GameplayStatics.GetPlayerController` 0)))
    (bind _output_get (set `self.Player Widget` _returnvalue))
    (`UserWidget.AddToViewport` _output_get 0)
    (bind _returnvalue_2 (`|CreateWidget` "/ItemSystem/UI/CraftingUI/WBP_PlayerCrafting.WBP_PlayerCrafting_C" null (`|MakeArray` (`self.BP_PlayerInventory`) :!type "InventoryComponent Object Reference") (`self.BP_PlayerCraftingComponent`)))
    (bind _output_get_2 (set `self.Player Inventory Widget` _returnvalue_2))
    (`/ItemSystem/UI/CraftingUI/WBP_PlayerCrafting.Set References` _output_get_2)))

(fn `Remove Menu`
  (params (`Target UI` :type "UserWidget Object Reference"))
  (if (== `Target UI` (`self.Active Widget`))
    (`Widget.RemoveFromParent` (`self.Active Widget`))
    (set `self.Active Widget` null)
    (else
      (`Widget.RemoveFromParent` (`local.Target UI`))))
  (bind _asplayer_controller (cast `PlayerController` (`self.GetController`)))
  (set `PlayerController.bShowMouseCursor` false _asplayer_controller)
  (`WidgetBlueprintLibrary.SetInputMode_GameOnly` _asplayer_controller))

(fn `UserConstructionScript`
  (`parent.UserConstructionScript`))